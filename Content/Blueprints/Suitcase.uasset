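; Suitcase pickup actor that any actor implementing the Playable interface collects by overlapping it.
; On spawn it deactivates its coin burst component and plays a 2D sound.
; Each tick it pulses the Box's scale uniformly with a sine wave over accumulated time.
; Collection spawns the coin burst at the component's transform, plays a coin sound at the world origin and destroys the actor.
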(event `self.ReceiveBeginPlay`
  (`ActorComponent.Deactivate` (`self.coinsBurst`))
  (`GameplayStatics.SpawnSound2D` "/Game/Audio/Valise_Angels_V2.Valise_Angels_V2" 1.0 1.0 0.0 null))

(event `self.ReceiveActorBeginOverlap`
  (params (OtherActor :type "Actor Object Reference"))
  (bind _coinsburst (`self.coinsBurst`))
  (if (`KismetSystemLibrary.DoesImplementInterface` OtherActor "/Game/Pawns/Playable.Playable_C")
    (`GameplayStatics.SpawnEmitterAtLocation` "/Game/ParticleSystems/coinsBurst.coinsBurst" (`SceneComponent.K2_GetComponentLocation` _coinsburst) (struct) (`SceneComponent.K2_GetComponentScale` _coinsburst))
    (`GameplayStatics.SpawnSoundAtLocation` "/Game/Audio/Coins.Coins" (0.0 0.0 0.0) (struct) 1.0 1.0 0.0 null null)
    (`self.K2_DestroyActor`)))

(event `self.ReceiveTick`
  (params (DeltaSeconds :type "Float (single-precision)"))
  (bind _returnvalue (+ (* DeltaSeconds (`self.GlowingSpeed`)) (`self.time`)))
  (bind _returnvalue_2 (+ (* (`KismetMathLibrary.Sin` _returnvalue) (`self.Amplitude`)) (`self.BaseScale`)))
  (`SceneComponent.SetWorldScale3D` (`self.Box`) (`KismetMathLibrary.MakeVector` _returnvalue_2 _returnvalue_2 _returnvalue_2))
  (set `self.time` _returnvalue))

(fn `UserConstructionScript`)